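; Character Blueprint for the Great arena character, with a chargeable attack and a timed dash ability.
; Holding attack plays a directional charge flipbook that resumes from a fixed frame whenever it ends, and release plays the attack flipbook, then finishes the attack.
; The dash drives velocity along Facing until its length elapses, then zeroes speed when the ability ends.
; Flipbooks are looked up in per-direction maps keyed by Facing.
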(event `self.AttackState`
  (params (AttackTime :type "Float (single-precision)") (AttackDown :type Boolean))
  ;[1 0.1557 0.1458] Attack State
  (if AttackDown
    (set `self.Charging` true)
    (`self.PlayFlipbook` (`BlueprintMapLibrary.Map_Find` (`self.ChargeAnimations`) (`self.Facing`)))
    (else
      (set `self.Charging` false)
      (`self.PlayFlipbook` (`BlueprintMapLibrary.Map_Find` (`self.AttackAnimations`) (`self.Facing`))))))

(event `self.AbilityEnd`
  ;[0.3118 1 0.4204] Dash End
  (`self.SetVelocity` 0.0 (`self.Facing`)))

(event `self.AbilityState`
  (params (AbilityTime :type "Float (single-precision)") (AbilityDown :type Boolean))
  ;[0.3118 1 0.4204] Dash State
  (if (< AbilityTime (`self.DashLength`))
    (`self.SetVelocity` (`self.DashSpeed`) (`self.Facing`))
    (`self.PlayFlipbook` (`BlueprintMapLibrary.Map_Find` (`self.DashAnimations`) (`self.Facing`)))
    (else
      (`self.FinishAbility`))))

(event `self.AnimationFinished`
  (bind _sprite (`self.Sprite`))
  (switch `CharacterState` (`self.CharacterState`)
    (:`Attacking`
      ;[1 1 1] Attack Animation Finished
      (if (`self.Charging`)
        (`PaperFlipbookComponent.SetPlaybackPositionInFrames` _sprite 22 false)
        (`PaperFlipbookComponent.Play` _sprite)
        (else
          (`self.FinishAttack`))))))

(fn `UserConstructionScript`
  (`parent.UserConstructionScript`))